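; Game mode for a Snake game that handles food spawning and the game-over screen.
; SpawnFood, first called on BeginPlay, places BP_Food at a random point inside the XMax/YMax bounds, inset by one cell and snapped to a 100-unit grid.
; GameOver shows the WBP_GameOver widget, pauses the game and switches input to UI-only with a visible mouse cursor.
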(event Custom|SpawnFood
  (bind _xmax (Variables|Default|GetXMax))
  (bind _ymax (Variables|Default|GetYMax))
  (bind _returnvalue (- _xmax 1e+02))
  (bind _returnvalue_2 (- _ymax 1e+02))
  (Game|SpawnActorfromClass "/Game/Blueprints/Snake/BP_Food.BP_Food_C" (Math|Transform|MakeTransform (Math|Vector|MakeVector (* (.ReturnValue (Math|Float|Division(WholeandRemainder) (Math|Random|RandomFloatinRange (* _returnvalue -1.0) _returnvalue) 1e+02)) 1e+02) (* (.ReturnValue (Math|Float|Division(WholeandRemainder) (Math|Random|RandomFloatinRange (* _returnvalue_2 -1.0) _returnvalue_2) 1e+02)) 1e+02) 5e+01) "0, 0, 0" "1.000000,1.000000,1.000000") "AdjustIfPossibleButAlwaysSpawn" "MultiplyWithRoot" 0 0))

(event Custom|GameOver
  (bind _returnvalue (UserInterface|CreateWidget "/Game/Blueprints/Snake/WBP_GameOver.WBP_GameOver_C" (Game|GetPlayerController 0)))
  (UserInterface|Viewport|AddtoViewport _returnvalue 0)
  (Game|SetGamePaused true)
  (Input|SetInputModeUIOnly (Game|GetPlayerController 0) _returnvalue "DoNotLock" false)
  (Variables|/Script/Engine.PlayerController|SetbShowMouseCursor (Game|GetPlayerController 0) true))

(event EventBeginPlay
  (CallFunction|SpawnFood))

(event EventTick
  (params (DeltaSeconds :type Float%20%28single-precision%29)))

(fn ConstructionScript)