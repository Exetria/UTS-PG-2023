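; BP_Food is the food pickup actor in the Snake game.
; Its PlayerOverlap event receives the player and calls EatFruit on it, asks GM_SnakeGameMode to spawn new food, then destroys itself.
; Its own overlap, BeginPlay and Tick events are disabled, and nothing in this Blueprint triggers PlayerOverlap.
; If the game mode cast fails, the food is neither replaced nor destroyed.
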(event EventBeginPlay
  (|CallParentFunction) ; This node is disabled and will not be called.\nDrag off pins to build functionality.
)

(event Collision|EventActorBeginOverlap
  (params (OtherActor :type Actor%20Object%20Reference))
  (|CallParentFunction OtherActor) ; This node is disabled and will not be called.\nDrag off pins to build functionality.
)

(event EventTick
  (params (DeltaSeconds :type Float%20%28single-precision%29))
  (|CallParentFunction DeltaSeconds) ; This node is disabled and will not be called.\nDrag off pins to build functionality.
)

(event EventPlayerOverlap
  (params (Player :type BP%20Head%20Object%20Reference))
  (Default|EatFruit Player)
  (bind _asgm_snake_game_mode (Utilities|Casting|CastToGM_SnakeGameMode (Game|GetGameMode)))
  (Default|SpawnFood _asgm_snake_game_mode)
  (Actor|DestroyActor))

(fn ConstructionScript
  (|CallParentFunction))