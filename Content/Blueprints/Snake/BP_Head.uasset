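; BP_Head is the player-steered head of a Snake game, growing a BP_Body segment whenever EatFruit fires.
; Each Tick it moves one mesh-width along the input direction, and tail segments shift into their predecessor's previous location.
; Direction inputs check the last actual movement to block reversing along the current axis.
; New segments copy the head's mesh at reduced scale, and the construction script places the head at world origin.
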(event Custom|AddTail
  (bind _returnvalue (Game|SpawnActorfromClass "/Game/Blueprints/Snake/BP_Body.BP_Body_C" (Math|Transform|MakeTransform (- (Transformation|GetActorLocation) (* (Variables|Default|GetMoveDIr) (Variables|Default|GetStepSize))) "0, 0, 0" "0.600000,0.600000,0.600000") "Undefined" "MultiplyWithRoot" 0 0))
  (Components|StaticMesh|SetStaticMesh (Variables|/Game/Blueprints/Snake/BP_KillerBlock.BP_KillerBlock_C|GetMesh _returnvalue) (Variables|/Script/Engine.StaticMeshComponent|GetStaticMesh (Variables|Default|GetHead)))
  (Utilities|Array|Add (Variables|Default|GetTails) _returnvalue))

(event Custom|EatFruit
  (CallFunction|AddTail))

(event EventBeginPlay
  (bind _head (Variables|Default|GetHead))
  (bind _staticmesh (Variables|/Script/Engine.StaticMeshComponent|GetStaticMesh _head))
  (bind _returnvalue (StaticMesh|GetBoundingBox _staticmesh))
  (Variables|Default|SetPreviousItemLocation (Transformation|GetActorLocation))
  (Variables|Default|SetStepSize (- (.x (.max _returnvalue)) (.x (.min _returnvalue)))))

(event Collision|EventActorBeginOverlap
  (params (OtherActor :type Actor%20Object%20Reference)))

(event EventTick
  (params (DeltaSeconds :type Float%20%28single-precision%29))
  (Variables|Default|SetPreviousItemLocation (Transformation|GetActorLocation))
  (Transformation|AddActorWorldOffset (* (Variables|Default|GetMoveDIr) (Variables|Default|GetStepSize)))
  (Variables|Default|SetCurMoveDir (- (Transformation|GetActorLocation) (Variables|Default|GetPreviousItemLocation)))
  (for _array_element (Variables|Default|GetTails)
    (bind _output_get (Variables|Default|SetCurTailLocation (Transformation|GetActorLocation _array_element)))
    (Transformation|SetActorLocation _array_element (Variables|Default|GetPreviousItemLocation) false false)
    (Variables|Default|SetPreviousItemLocation _output_get)))

(event Input|ActionEvents|InputActionMoveUp
  (params (Key :type Key%20Structure :default "None"))
  (:Pressed
    (if (== (.x (Variables|Default|GetCurMoveDir)) 0.0)
      (Variables|Default|SetMoveDIr "1.000000,0.000000,0.000000"))))

(event Input|ActionEvents|InputActionMoveDown
  (params (Key :type Key%20Structure :default "None"))
  (:Pressed
    (if (== (.x (Variables|Default|GetCurMoveDir)) 0.0)
      (Variables|Default|SetMoveDIr "-1.000000,0.000000,0.000000"))))

(event Input|ActionEvents|InputActionMoveRight
  (params (Key :type Key%20Structure :default "None"))
  (:Pressed
    (if (== (.y (Variables|Default|GetCurMoveDir)) 0.0)
      (Variables|Default|SetMoveDIr "0.000000,1.000000,0.000000"))))

(event Input|ActionEvents|InputActionMoveLeft
  (params (Key :type Key%20Structure :default "None"))
  (:Pressed
    (if (== (.y (Variables|Default|GetCurMoveDir)) 0.0)
      (Variables|Default|SetMoveDIr "0.000000,-1.000000,0.000000"))))

(fn ConstructionScript
  (Transformation|SetActorLocation "0, 0, 0" false false))