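; Unblocked-style sliding block puzzle on a 3x3 grid, with single cubes and a two-cell horizontal arrow block.
; The construction script spawns cubes and text markers from the Numbers array, where zero is empty.
; Debug arrow keys move the selection marker, while WASD slides the selected piece by swapping array entries.
; Update refreshes visuals and runs CheckResult, which tests the arrow block's bottom-row position for a win reported through PrintString.
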(event Input|KeyboardEvents|DebugKeyA
  (params (Key :type Key%20Structure :default "None") (ActionValue :type Input%20Action%20Value%20Structure))
  (:Pressed
    (Variables|Default|SetmoveDirection 2)
    (CallFunction|Move)))

(event Input|KeyboardEvents|DebugKeyS
  (params (Key :type Key%20Structure :default "None") (ActionValue :type Input%20Action%20Value%20Structure))
  (:Pressed
    (Variables|Default|SetmoveDirection 3)
    (CallFunction|Move)))

(event Input|KeyboardEvents|DebugKeyD
  (params (Key :type Key%20Structure :default "None") (ActionValue :type Input%20Action%20Value%20Structure))
  (:Pressed
    (Variables|Default|SetmoveDirection 4)
    (CallFunction|Move)))

(event Input|KeyboardEvents|DebugKeyUp
  (params (Key :type Key%20Structure :default "None") (ActionValue :type Input%20Action%20Value%20Structure))
  (:Pressed
    (Variables|Default|SetselectionMoveDirection 1)
    (CallFunction|MoveSelected)))

(event Input|KeyboardEvents|DebugKeyLeft
  (params (Key :type Key%20Structure :default "None") (ActionValue :type Input%20Action%20Value%20Structure))
  (:Pressed
    (Variables|Default|SetselectionMoveDirection 2)
    (CallFunction|MoveSelected)))

(event Input|KeyboardEvents|DebugKeyDown
  (params (Key :type Key%20Structure :default "None") (ActionValue :type Input%20Action%20Value%20Structure))
  (:Pressed
    (Variables|Default|SetselectionMoveDirection 3)
    (CallFunction|MoveSelected)))

(event Input|KeyboardEvents|DebugKeyRight
  (params (Key :type Key%20Structure :default "None") (ActionValue :type Input%20Action%20Value%20Structure))
  (:Pressed
    (Variables|Default|SetselectionMoveDirection 4)
    (CallFunction|MoveSelected)))

(event Input|KeyboardEvents|DebugKeyW
  (params (Key :type Key%20Structure :default "None") (ActionValue :type Input%20Action%20Value%20Structure))
  (:Pressed
    (Variables|Default|SetmoveDirection 1)
    (CallFunction|Move)))

(fn ConstructionScript
  (bind _dimension (Variables|Default|Getdimension))
  (for _index (range 0 (- (Utilities|Array|Length (Variables|Default|Getnumbers)) 1))
    (bind _returnvalue (AddComponent|AddStaticMeshComponent false (Math|Transform|MakeTransform (Math|Vector|MakeVector (Math|Conversions|ToFloat(Integer) (* (Math|Integer|%(Integer) _index _dimension) 200)) 0.0 (Math|Conversions|ToFloat(Integer) (+ (* (/ _index _dimension) -200) 600))) "0, 0, 0" "1.000000,1.000000,1.000000")))
    (Utilities|Array|Add (Variables|Default|Getcubes) _returnvalue)
    (bind _returnvalue_2 (AddComponent|AddTextRenderComponent false (Math|Transform|MakeTransform (Math|Vector|MakeVector (Math|Conversions|ToFloat(Integer) (* (Math|Integer|%(Integer) _index _dimension) 200)) 100.1 (Math|Conversions|ToFloat(Integer) (+ (* (/ _index _dimension) -200) 600))) "0.000000,90.000000,0.000000" "1.000000,1.000000,1.000000")))
    (Utilities|Array|Add (Variables|Default|Gettexts) _returnvalue_2)
    (if (== (Utilities|Array|Get(acopy) (Variables|Default|Getnumbers) _index) 0)
      (Rendering|SetVisibility (Utilities|Array|Get(acopy) (Variables|Default|Getcubes) _index) false false)
      (elif (or (== (Utilities|Array|Get(acopy) (Variables|Default|Getnumbers) _index) 2) (== (Utilities|Array|Get(acopy) (Variables|Default|Getnumbers) _index) 3))
        (Rendering|Material|SetMaterial (Utilities|Array|Get(acopy) (Variables|Default|Getcubes) _index) 0 "/Engine/VREditor/UI/ArrowMaterial.ArrowMaterial")))
    (Rendering|SetVisibility (Utilities|Array|Get(acopy) (Variables|Default|Gettexts) _index) false false)
    (Variables|Default|Setselected 0)
    (Rendering|SetVisibility (Utilities|Array|Get(acopy) (Variables|Default|Gettexts)) true false)))

(fn CheckResult
  (bind _numbers (Variables|Default|Getnumbers))
  (bind _output (Utilities|Array|Get(acopy) _numbers 6))
  (bind (_array_element _array_index) (Utilities|Array|ForEachLoopwithBreak (Variables|Default|Getnumbers) :!label _label)
    (:LoopBody
      (if (== _array_element 2)
        (if (== (/ _array_index 3) 2)
          (if (or (== _output 0) (== _output 2))
            (Variables|Default|Setresult true)
            (goto _label Break))
          (else
            (Variables|Default|Setresult false :!label _label_2)))
        (else
          (goto _label_2))))))

(fn Update
  (for _index (range 0 (- (Utilities|Array|Length (Variables|Default|Getnumbers)) 1))
    (if (or (== (Utilities|Array|Get(acopy) (Variables|Default|Getnumbers) _index) 2) (== (Utilities|Array|Get(acopy) (Variables|Default|Getnumbers) _index) 3))
      (Rendering|Material|SetMaterial (Utilities|Array|Get(acopy) (Variables|Default|Getcubes) _index) 0 "/Engine/VREditor/UI/ArrowMaterial.ArrowMaterial")
      (else
        (Rendering|Material|SetMaterial (Utilities|Array|Get(acopy) (Variables|Default|Getcubes) _index) 0 "/Engine/EngineMaterials/WorldGridMaterial.WorldGridMaterial")))
    (if (== (Utilities|Array|Get(acopy) (Variables|Default|Getnumbers) _index) 0)
      (Rendering|SetVisibility (Utilities|Array|Get(acopy) (Variables|Default|Getcubes) _index) false false)
      (else
        (Rendering|SetVisibility (Utilities|Array|Get(acopy) (Variables|Default|Getcubes) _index) true false)))
    (if (== _index (Variables|Default|Getselected))
      (Rendering|SetVisibility (Utilities|Array|Get(acopy) (Variables|Default|Gettexts) _index) true false)
      (else
        (Rendering|SetVisibility (Utilities|Array|Get(acopy) (Variables|Default|Gettexts) _index) false false)))
    (CallFunction|CheckResult)))

(fn Move
  (bind _movedirection (Variables|Default|GetmoveDirection))
  (bind _numbers (Variables|Default|Getnumbers))
  (bind _numbers_2 (Variables|Default|Getnumbers))
  (bind _numbers_3 (Variables|Default|Getnumbers))
  (bind _numbers_4 (Variables|Default|Getnumbers))
  (bind _numbers_5 (Variables|Default|Getnumbers))
  (bind _movedirection_2 (Variables|Default|GetmoveDirection))
  (if (== (Utilities|Array|Get(acopy) (Variables|Default|Getnumbers) (Variables|Default|Getselected)) 1)
    (if (== _movedirection_2 3)
      (if (<= (+ (Variables|Default|Getselected) 3) 8)
        (Variables|Default|SetswapTarget (+ (Variables|Default|Getselected) 3))
        (if (== (Utilities|Array|Get(acopy) (Variables|Default|Getnumbers) (Variables|Default|GetswapTarget)) 0) :!label _label
          (Utilities|Array|Swap (Variables|Default|Getnumbers) (Variables|Default|Getselected) (Variables|Default|GetswapTarget))
          (Variables|Default|Setselected (Variables|Default|GetswapTarget))
          (CallFunction|Update)
          (if (Variables|Default|Getresult)
            (Development|PrintString "=====MENANGGGGG=====")
            (else
              (Development|PrintString "=====Belum Benar====="))))
        (else
          (Development|PrintString "Cannot Move!!" :!label _label_2)))
      (elif (== _movedirection_2 4)
        (if (and (< (+ (Variables|Default|Getselected) 1) 9) (== (/ (+ (Variables|Default|Getselected) 1) 3) (/ (Variables|Default|Getselected) 3)))
          (Variables|Default|SetswapTarget (+ (Variables|Default|Getselected) 1))
          (Development|PrintString "Moved Right")
          (goto _label)
          (else
            (goto _label_2)))
        (elif (== _movedirection_2 1)
          (if (>= (- (Variables|Default|Getselected) 3) 0)
            (Variables|Default|SetswapTarget (- (Variables|Default|Getselected) 3))
            (goto _label)
            (else
              (goto _label_2)))
          (elif (== _movedirection_2 2)
            (if (and (== (/ (- (Variables|Default|Getselected) 1) 3) (/ (Variables|Default|Getselected) 3)) (> (- (Variables|Default|Getselected) 1) -1))
              (Variables|Default|SetswapTarget (- (Variables|Default|Getselected) 1))
              (Development|PrintString "Moved Left")
              (goto _label)
              (else
                (goto _label_2)))))))
    (elif (> (Utilities|Array|Get(acopy) (Variables|Default|Getnumbers) (Variables|Default|Getselected)) 1)
      (if (== (Utilities|Array|Get(acopy) (Variables|Default|Getnumbers) (Variables|Default|Getselected)) 2)
        _
        (else
          (Variables|Default|SetselectionMoveDirection 2)
          (CallFunction|MoveSelected)))
      (if (== _movedirection 1)
        (if (>= (- (Variables|Default|Getselected) 3) 0)
          (Variables|Default|SetswapTarget (- (Variables|Default|Getselected) 3))
          (if (and (== (Utilities|Array|Get(acopy) _numbers_5 (Variables|Default|GetswapTarget)) 0) (== (Utilities|Array|Get(acopy) _numbers_5 (- (Variables|Default|GetswapTarget) 0)) 0))
            (Utilities|Array|Swap _numbers_4 (Variables|Default|Getselected) (Variables|Default|GetswapTarget))
            (Utilities|Array|Swap _numbers_4 (+ (Variables|Default|Getselected) 1) (+ (Variables|Default|GetswapTarget) 1))
            (Variables|Default|Setselected (Variables|Default|GetswapTarget) :!label _label_3)
            (CallFunction|Update)
            (if (Variables|Default|Getresult)
              (Development|PrintString "=====MENANGGGGG=====")
              (else
                (Development|PrintString "=====Belum Benar=====")))))
        (elif (== _movedirection 2)
          (if (and (== (/ (Variables|Default|Getselected) 3) (/ (- (Variables|Default|Getselected) 1) 3)) (> (- (Variables|Default|Getselected) 1) -1))
            (Variables|Default|SetswapTarget (- (Variables|Default|Getselected) 1))
            (if (== (Utilities|Array|Get(acopy) (Variables|Default|Getnumbers) (Variables|Default|GetswapTarget)) 0)
              (Utilities|Array|Swap _numbers (Variables|Default|Getselected) (Variables|Default|GetswapTarget))
              (Utilities|Array|Swap _numbers (+ (Variables|Default|Getselected) 1) (Variables|Default|Getselected))
              (Development|PrintString "Moved Left")
              (goto _label_3)))
          (elif (== _movedirection 3)
            (if (<= (+ (Variables|Default|Getselected) 3) 8)
              (Variables|Default|SetswapTarget (+ (Variables|Default|Getselected) 3))
              (if (and (== (Utilities|Array|Get(acopy) _numbers_2 (Variables|Default|GetswapTarget)) 0) (== (Utilities|Array|Get(acopy) _numbers_2 (+ (Variables|Default|GetswapTarget) 1)) 0))
                (Utilities|Array|Swap _numbers_3 (Variables|Default|Getselected) (Variables|Default|GetswapTarget))
                (Utilities|Array|Swap _numbers_3 (+ (Variables|Default|Getselected) 1) (+ (Variables|Default|GetswapTarget) 1))
                (goto _label_3)))
            (elif (== _movedirection 4)
              (if (and (< (+ (Variables|Default|Getselected) 2) 9) (== (/ (+ (Variables|Default|Getselected) 2) 3) (/ (Variables|Default|Getselected) 3)))
                (Variables|Default|SetswapTarget (+ (Variables|Default|Getselected) 2))
                (if (== (Utilities|Array|Get(acopy) (Variables|Default|Getnumbers) (Variables|Default|GetswapTarget)) 0)
                  (Utilities|Array|Swap _numbers (+ (Variables|Default|Getselected) 1) (Variables|Default|GetswapTarget))
                  (Utilities|Array|Swap _numbers (Variables|Default|Getselected) (+ (Variables|Default|Getselected) 1))
                  (Development|PrintString "Moved Right")
                  (Variables|Default|SetswapTarget (- (Variables|Default|GetswapTarget) 1))
                  (goto _label_3))))))))))

(fn MoveSelected
  (bind _texts (Variables|Default|Gettexts))
  (bind _texts_2 (Variables|Default|Gettexts))
  (bind _selectionmovedirection (Variables|Default|GetselectionMoveDirection))
  (if (== _selectionmovedirection 1)
    (if (>= (- (Variables|Default|Getselected) 3) 0)
      (Rendering|SetVisibility (Utilities|Array|Get(acopy) _texts (- (Variables|Default|Getselected) 3)) true false)
      (Rendering|SetVisibility (Utilities|Array|Get(acopy) _texts (Variables|Default|Getselected)) false false)
      (Variables|Default|Setselected (- (Variables|Default|Getselected) 3)))
    (elif (== _selectionmovedirection 3)
      (if (<= (+ (Variables|Default|Getselected) 3) 8)
        (Rendering|SetVisibility (Utilities|Array|Get(acopy) _texts (+ (Variables|Default|Getselected) 3)) true false)
        (Rendering|SetVisibility (Utilities|Array|Get(acopy) _texts (Variables|Default|Getselected)) false false)
        (Variables|Default|Setselected (+ (Variables|Default|Getselected) 3)))
      (elif (== _selectionmovedirection 2)
        (if (and (!= (Variables|Default|Getselected) 0) (== (/ (- (Variables|Default|Getselected) 1) 3) (/ (Variables|Default|Getselected) 3)))
          (Rendering|SetVisibility (Utilities|Array|Get(acopy) _texts_2 (- (Variables|Default|Getselected) 1)) true false)
          (Rendering|SetVisibility (Utilities|Array|Get(acopy) _texts_2 (Variables|Default|Getselected)) false false)
          (Variables|Default|Setselected (- (Variables|Default|Getselected) 1)))
        (elif (== _selectionmovedirection 4)
          (if (and (== (/ (+ (Variables|Default|Getselected) 1) 3) (/ (Variables|Default|Getselected) 3)) (!= (Variables|Default|Getselected) 8))
            (Rendering|SetVisibility (Utilities|Array|Get(acopy) _texts_2 (+ (Variables|Default|Getselected) 1)) true false)
            (Rendering|SetVisibility (Utilities|Array|Get(acopy) _texts_2 (Variables|Default|Getselected)) false false)
            (Variables|Default|Setselected (+ (Variables|Default|Getselected) 1))))))))