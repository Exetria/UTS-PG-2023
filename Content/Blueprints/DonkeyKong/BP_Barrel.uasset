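; Barrel hazard for the Donkey Kong game that damages the player character on contact.
; On BeginPlay, a physics impulse on its Cylinder launches it along world +Y.
; Both overlap and hit events on the Cylinder cast to BP_Donkey_Kong_Character, apply damage, then destroy the barrel, ignoring other actors.
; Any damage the barrel receives also destroys it.
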(event OnComponentBeginOverlap(Cylinder)
  (params (OverlappedComponent :type Primitive%20Component%20Object%20Reference) (OtherActor :type Actor%20Object%20Reference) (OtherComp :type Primitive%20Component%20Object%20Reference) (OtherBodyIndex :type Integer) (bFromSweep :type Boolean) (SweepResult :type Hit%20Result%20Structure%20%28by%20ref%29))
  (bind _asbp_donkey_kong_character (Utilities|Casting|CastToBP_Donkey_Kong_Character OtherActor))
  (Game|Damage|ApplyDamage _asbp_donkey_kong_character 1.0 0 0)
  (Actor|DestroyActor))

(event OnComponentHit(Cylinder)
  (params (HitComponent :type Primitive%20Component%20Object%20Reference) (OtherActor :type Actor%20Object%20Reference) (OtherComp :type Primitive%20Component%20Object%20Reference) (NormalImpulse :type Vector :default "0, 0, 0") (Hit :type Hit%20Result%20Structure%20%28by%20ref%29))
  (bind _asbp_donkey_kong_character (Utilities|Casting|CastToBP_Donkey_Kong_Character OtherActor))
  (Game|Damage|ApplyDamage _asbp_donkey_kong_character 1.0 0 0)
  (Actor|DestroyActor))

(event EventBeginPlay
  (Physics|AddImpulse (Variables|Default|GetCylinder) "0.000000,1000.000000,0.000000" "None" false))

(event EventTick
  (params (DeltaSeconds :type Float%20%28single-precision%29)))

(event Game|Damage|EventAnyDamage
  (params (Damage :type Float%20%28single-precision%29) (DamageType :type Damage%20Type%20Object%20Reference) (InstigatedBy :type Controller%20Object%20Reference) (DamageCauser :type Actor%20Object%20Reference))
  (Actor|DestroyActor))

(fn ConstructionScript)